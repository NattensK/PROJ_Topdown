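; Arrow projectile fired from the player's bow that homes in on a saved enemy target and deals damage on impact.
; BeginPlay takes the target from the player combat bow component, sets it as homing target and clears the component's copy.
; A millisecond looping timer re-aims velocity at the enemy while valid.
; Impact, bound in construction like RotateToTarget, stops the timer, sends a damage message and destroys the arrow.
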(event Custom|RotateToTarget
  (bind _returnvalue (Utilities|Time|SetTimerbyEvent (delegate Custom|RotateToTarget) 0.001 true))
  (Variables|Default|SetTimerHandle _returnvalue)
  (bind _saved_target_enemy (Variables|Default|GetSaved%20Target%20Enemy)
    (:then
      (Variables|/Script/Engine.MovementComponent|SetVelocity (Variables|Default|GetProjectileMovement) (* (Math|Vector|GetUnitDirection(Vector) (Transformation|GetActorLocation) (Transformation|GetActorLocation _saved_target_enemy)) (Variables|Default|GetSpeed))))
    (:else)))

(event Custom|ProjectileImpact
  (params (Other%20Actor :type Actor%20Object%20Reference) (Hit :type Hit%20Result%20Structure) (SDamageInfo :type S%20Damage%20Info%20Structure))
  (Variables|Default|SetSaved%20Target%20Enemy 0)
  (Utilities|Time|ClearandInvalidateTimerbyHandle (Variables|Default|GetTimerHandle))
  (Class|BPIDamagable|DealDamage(Message) Other%20Actor SDamageInfo)
  (Actor|DestroyActor))

(event EventBeginPlay
  (|CallParentFunction)
  (Default|CallOnRotatetoTarget)
  (bind _savedtargetenemy (Variables|/Game/Player/Blueprints/BPC_PlayerBow.BPC_PlayerBow_C|GetSavedTargetEnemy (Variables|/Game/Player/Blueprints/BPC_PlayerCombat.BPC_PlayerCombat_C|GetBPC_PlayerBow (Variables|Default|GetBPC_PlayerCombat)))
    (:then
      (Variables|/Script/Engine.ProjectileMovementComponent|SetHomingTargetComponent (Variables|Default|GetProjectileMovement) (Variables|/Script/Engine.Actor|GetRootComponent _savedtargetenemy))
      (Variables|Default|SetSaved%20Target%20Enemy _savedtargetenemy)
      (Variables|/Game/Player/Blueprints/BPC_PlayerBow.BPC_PlayerBow_C|SetSavedTargetEnemy (Variables|/Game/Player/Blueprints/BPC_PlayerCombat.BPC_PlayerCombat_C|GetBPC_PlayerBow (Variables|Default|GetBPC_PlayerCombat)) 0))
    (:else)))

(event Collision|EventActorBeginOverlap
  (params (OtherActor :type Actor%20Object%20Reference))
  (|CallParentFunction OtherActor) ; This node is disabled and will not be called.\nDrag off pins to build functionality.
)

(fn ConstructionScript
  (bind _self self)
  (|CallParentFunction)
  (Variables|Default|SetSpeed (Variables|Default|GetSpeed))
  (EventDispatchers|BindEventtoOnRotatetoTarget _self (EventDispatchers|CreateEvent :!event Custom|RotateToTarget))
  (EventDispatchers|BindEventtoOnProjectileImpact _self (EventDispatchers|CreateEvent :!event Custom|ProjectileImpact)))