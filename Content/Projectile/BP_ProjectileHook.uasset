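; Player hook projectile that launches toward the mouse position from the hook shoot point.
; On hitting an enemy, it deals damage, notifies the player's hook component and attaches to that enemy.
; Other impacts end the hook and destroy the projectile after a short delay.
; Damage info passes through CalculateStunDuration, whose graph holds distance-based stun scaling shown as unused.
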(event Custom|RotateToTarget
  (bind _direction (CallFunction|FindMousePosition (Variables|/Game/Player/Blueprints/BP_PlayerCharacter.BP_PlayerCharacter_C|GetHookShootPoint (Variables|Default|GetBP_PlayerCharacter))))
  (Variables|/Script/Engine.MovementComponent|SetVelocity (Variables|Default|GetProjectileMovement) (* _direction (Variables|Default|GetSpeed))))

(event Custom|ProjectileImpact
  (params (Other%20Actor :type Actor%20Object%20Reference) (Hit :type Hit%20Result%20Structure) (SDamageInfo :type S%20Damage%20Info%20Structure))
  (bind _bpc_playercombat (Variables|Default|GetBPC_PlayerCombat))
  (bind _bpc_playerhook (Variables|/Game/Player/Blueprints/BPC_PlayerCombat.BPC_PlayerCombat_C|GetBPC_PlayerHook _bpc_playercombat))
  (if (Class|GameplayStatics|ObjectIsA Other%20Actor "/Game/Enemies/Blueprints/BP_EnemyBase.BP_EnemyBase_C")
    (Class|BPIDamagable|DealDamage(Message) Other%20Actor (Utilities|CalculateStunDuration SDamageInfo))
    (Default|HookLanded _bpc_playerhook Other%20Actor)
    (Transformation|AttachActorToActor Other%20Actor "None" "SnapToTarget" "KeepWorld" "KeepWorld" true)
    (else
      (Default|HookFinished _bpc_playerhook)
      (Utilities|FlowControl|Delay 0.6)
      (Actor|DestroyActor))))

(event EventBeginPlay
  (|CallParentFunction)
  (Default|CallOnRotatetoTarget))

(event Collision|EventActorBeginOverlap
  (params (OtherActor :type Actor%20Object%20Reference))
  (|CallParentFunction OtherActor) ; This node is disabled and will not be called.\nDrag off pins to build functionality.
)

(fn ConstructionScript
  (bind _self self)
  (|CallParentFunction)
  (Variables|Default|SetSpeed (Variables|Default|GetSpeed))
  (EventDispatchers|BindEventtoOnRotatetoTarget _self (EventDispatchers|CreateEvent :!event Custom|RotateToTarget))
  (EventDispatchers|BindEventtoOnProjectileImpact _self (EventDispatchers|CreateEvent :!event Custom|ProjectileImpact)))

(fn FindMousePosition
  (params (SceneComponent :type Scene%20Component%20Object%20Reference))
  (bind _direction (|CallParentFunction SceneComponent))
  (return _direction))