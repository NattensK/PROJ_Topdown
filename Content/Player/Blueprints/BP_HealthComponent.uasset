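; Player health component that tracks Health and applies incoming damage through a TakeDamage event.
; Each accepted hit subtracts from Health, prints the new value and fires the OnDamageTaken dispatcher.
; A DoOnce gate reopens after a short delay, giving a brief invulnerability window between hits.
; At zero or below it fires the death dispatcher and leaves the gate closed, so later damage is ignored.
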(event Custom|TakeDamage
  (params (Amount :type Float%20%28double-precision%29))
  (Utilities|FlowControl|DoOnce false :!label _label
    (:Completed
      (bind _output_get (Variables|Default|SetHealth (- (Variables|Default|GetHealth) Amount)))
      (Development|PrintString (Utilities|String|ToString(Float) _output_get))
      (Default|CallOnDamageTaken)
      (if (<= _output_get 0.0)
        (Default|CallCallonDeath)
        (else
          (Utilities|FlowControl|Delay 0.8)
          (goto _label Reset))))))

(event EventBeginPlay)

(event EventTick
  (params (DeltaSeconds :type Float%20%28single-precision%29)))