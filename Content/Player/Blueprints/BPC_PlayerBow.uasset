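; Player bow component, built on a parent weapon component, that handles ranged attacks on the targeted enemy.
; Attack checks require combat readiness, grounded movement and a target within range, briefly showing a Niagara max-range circle when the target is too far.
; Attacks disable movement input, face the mouse and play a montage, whose animation triggers an arrow with randomized damage.
; Finishing re-enables attacking and clears the target if it is no longer hovered.
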(event Custom|SpawnProjectile
  (bind _bp_playercharacter (Variables|Default|GetBP_PlayerCharacter))
  (bind _bp_playercharacter_2 (Variables|Default|GetBP_PlayerCharacter))
  ;[0.05098 0.05098 0.05098] SpawnProjectile (from animation)
  (bind _returnvalue (Game|SpawnActorfromClass "/Game/Projectile/BP_ProjectileArrow.BP_ProjectileArrow_C" (Transformation|GetWorldTransform (Variables|/Game/Player/Blueprints/BP_PlayerCharacter.BP_PlayerCharacter_C|GetBowShootPoint _bp_playercharacter)) "Undefined" "MultiplyWithRoot" _bp_playercharacter 2.2e+03 0.1 false (Utilities|Struct|MakeS_DamageInfo (Math|Random|RandomFloatinRange 7.0 2e+01) "NewEnumerator1" "NewEnumerator2" "NewEnumerator0" "NewEnumerator1") false 0 0))
  (Collision|IgnoreActorwhenMoving (Variables|/Script/Engine.Character|GetCapsuleComponent _bp_playercharacter_2) _returnvalue true)
  (Collision|IgnoreActorwhenMoving (Variables|/Game/Projectile/BP_ProjectileBase.BP_ProjectileBase_C|GetBoxCollision _returnvalue) _bp_playercharacter_2 true))

(event Custom|ToggleMaxRangeCircle
  (bind _bp_playercharacter (Variables|Default|GetBP_PlayerCharacter))
  (bind _returnvalue (Actor|GetComponentbyClass _bp_playercharacter "/Script/Niagara.NiagaraComponent"))
  ;[0.05098 0.05098 0.05098] MaxRangeVisibility
  (if (Components|ComponentHasTag _returnvalue "MaxRangeCircle")
    (Rendering|SetVisibility _returnvalue true false)
    (Utilities|FlowControl|RetriggerableDelay 1.4)
    (Rendering|SetVisibility _returnvalue false false)))

(event Custom|BowAttack
  ;[0.05098 0.05098 0.05098] Attack
  (Variables|/Game/Player/Blueprints/BPC_PlayerCombat.BPC_PlayerCombat_C|SetIsAttacking (Variables|Default|GetBPC_PlayerBow) true)
  (Default|ToggleEnableMovementInput (Variables|Default|GetBP_PlayerCharacter) false true)
  (Default|RotateTowardsMouse (Variables|Default|GetBPC_PlayerCombat))
  (Animation|Montage|PlayMontage (Variables|Default|GetPlayerMesh) (Utilities|Array|Get(acopy) (Variables|Default|GetattackAnims) 1) 7.0))

(event EventBeginPlay
  (bind _bp_playercharacter (Variables|Default|GetBP_PlayerCharacter))
  (bind _returnvalue (Actor|GetComponentbyClass _bp_playercharacter "/Script/Niagara.NiagaraComponent"))
  ;[0.05098 0.05098 0.05098] Setup
  (|CallParentFunction)
  (Variables|Default|SetBow (Variables|/Game/Player/Blueprints/BP_PlayerCharacter.BP_PlayerCharacter_C|GetBow (Variables|Default|GetBP_PlayerCharacter)))
  (if (Components|ComponentHasTag _returnvalue "MaxRangeCircle")
    (Rendering|SetVisibility _returnvalue false false)))

(fn CheckCanAttack
  (bind _canattack (|CallParentFunction))
  (if _canattack
    (if (Variables|/Game/Player/Blueprints/BPC_PlayerCombat.BPC_PlayerCombat_C|GetCanAttack (Variables|Default|GetBPC_PlayerCombat))
      (if (AI|Components|NavMovement|IsMovingonGround (Variables|Default|GetCharacterMovement))
        (bind (_targettedenemy _enemylocation) (Default|GetTargettedEnemy (Variables|Default|GetBPC_PlayerCombat)))
        (Utilities|IsValid _targettedenemy
          (:Is%20Valid
            (if (<= (Math|Vector|Distance(Vector) _enemylocation (Transformation|GetActorLocation (Variables|Default|GetBP_PlayerCharacter))) (Variables|Default|GetMaxRange))
              (Variables|Default|SetSavedTargetEnemy _targettedenemy)
              (return true)
              (else
                (CallFunction|ToggleMaxRangeCircle self))))
          (:Is%20Not%20Valid
            _)))))
  (return false))

(fn HandleFinishedAttacking
  (bind _bpc_playercombat (Variables|Default|GetBPC_PlayerCombat))
  (Variables|/Game/Player/Blueprints/BPC_PlayerCombat.BPC_PlayerCombat_C|SetCanAttack (Variables|Default|GetBPC_PlayerBow) true)
  (bind _asbp_enemy_base (Utilities|Casting|CastToBP_EnemyBase (Variables|/Game/Player/Blueprints/BPC_PlayerCombat.BPC_PlayerCombat_C|GetTargettedEnemy _bpc_playercombat)))
  (if (not (Variables|/Game/Enemies/Blueprints/BP_EnemyBase.BP_EnemyBase_C|GetIsMouseHovering _asbp_enemy_base))
    (Default|SetTargettedEnemy _bpc_playercombat)
    (|CallParentFunction)))