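; Player combat component that routes attack inputs to the melee, bow and hook components and swaps the visible weapon mesh.
; Handler macros gate attacks through shared CanAttack and IsAttacking flags, with hook firing its projectile on release.
; Helpers rotate the player toward the cursor, a set target, or the closest enemy in a sphere ahead.
; Number keys trigger debug enemy states, damage and montage tests.
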(event Custom|FinishedAttacking
  ;[0.05098 0.05098 0.05098] Finished attacking
  (switch Utilities|FlowControl|Switch|Switchone_WeaponType (Variables|WeaponType|GetWeaponType)
    (:NewEnumerator1
      (CallFunction|HandleFinishedAttacking (Variables|Default|GetBPC_PlayerMelee)))
    (:NewEnumerator2
      (CallFunction|HandleFinishedAttacking (Variables|Default|GetBPC_PlayerBow)))
    (:NewEnumerator3
      (CallFunction|HandleFinishedAttacking (Variables|Default|GetBPC_PlayerHook)))))

(event EventBeginPlay
  ;[0.05098 0.05098 0.05098] Setup
  (Utilities|GetActorComponents)
  (Utilities|GetMeshes)
  (Variables|BPC_PlayerCombat_C|SetPreviousWeapon (Variables|Default|GetBPC_PlayerCombat) (.Value (Utilities|Map|Find (Variables|WeaponType|GetWeaponMeshes) "NewEnumerator2")))
  (CallFunction|ChangeWeaponType))

(event Input|ActionEvents|InputActionHook
  (params (Key :type Key%20Structure :default "None"))
  ;[0.05098 0.05098 0.05098] Check if attack is allowed & sets "attack style" depending on input
  (:Pressed
    (Utilities|CanReleaseAttackHandler (Variables|Default|GetBPC_PlayerHook) :!label _label
      (:OnPress
        (Variables|WeaponType|SetWeaponType "NewEnumerator3")
        (Default|HookAttack (Variables|Default|GetBPC_PlayerHook))
        (CallFunction|ChangeWeaponType)
        (Variables|BPC_PlayerCombat_C|SetIsAttacking (Variables|Default|GetBPC_PlayerCombat) true))
      (:OnRelease
        (Default|SpawnProjectile (Variables|Default|GetBPC_PlayerHook)))))
  (:Released
    (goto _label Released)))

(event Input|ActionEvents|InputActionRangedAttack
  (params (Key :type Key%20Structure :default "None"))
  ;[0.05098 0.05098 0.05098] Check if attack is allowed & sets "attack style" depending on input
  (:Pressed
    (Utilities|CanAttackHandler (Variables|Default|GetBPC_PlayerBow)
      (:OnPress
        (Variables|WeaponType|SetWeaponType "NewEnumerator2")
        (Default|BowAttack (Variables|Default|GetBPC_PlayerBow))
        (CallFunction|ChangeWeaponType)
        (Variables|BPC_PlayerCombat_C|SetIsAttacking (Variables|Default|GetBPC_PlayerCombat) true)))))

(event Input|ActionEvents|InputActionAttack
  (params (Key :type Key%20Structure :default "None"))
  ;[0.05098 0.05098 0.05098] Check if attack is allowed & sets "attack style" depending on input
  (:Pressed
    (Utilities|CanAttackHandler (Variables|Default|GetBPC_PlayerMelee)
      (:OnPress
        (Variables|WeaponType|SetWeaponType "NewEnumerator1")
        (Default|MeleeAttack (Variables|Default|GetBPC_PlayerMelee))
        (CallFunction|ChangeWeaponType)
        (Variables|BPC_PlayerCombat_C|SetIsAttacking (Variables|Default|GetBPC_PlayerCombat) true)))))

(event Input|KeyboardEvents|3
  (params (Key :type Key%20Structure :default "None"))
  ;[0.05098 0.05098 0.05098] debugging
  (:Pressed
    (bind _returnvalue (Actor|GetActorOfClass "/Game/Enemies/Blueprints/BP_EnemyBase.BP_EnemyBase_C"))
    (bind _returnvalue_2 (Actor|GetActorOfClass "/Game/Player/Blueprints/BP_PlayerCharacter.BP_PlayerCharacter_C"))
    (Class|AISenseDamage|ReportDamageEvent _returnvalue _returnvalue_2 0.0 "0, 0, 0" "0, 0, 0" "None")
    (Default|DealDamage _returnvalue)))

(event Input|KeyboardEvents|5
  (params (Key :type Key%20Structure :default "None"))
  ;[0.05098 0.05098 0.05098] debugging
  (:Pressed
    (Animation|Montage|PlayMontage (Variables|Default|GetPlayerMesh) (Utilities|Array|Get(acopy) (Variables|/Game/Player/Blueprints/BPC_PlayerMelee.BPC_PlayerMelee_C|GetattackAnims (Variables|Default|GetBPC_PlayerMelee)) 2) 3.5) ; 2.4
  ))

(event Input|KeyboardEvents|2
  (params (Key :type Key%20Structure :default "None"))
  ;[0.05098 0.05098 0.05098] debugging
  (:Pressed
    (bind _outactors (Actor|GetAllActorsOfClass "/Game/Enemies/Blueprints/BP_EnemyBase.BP_EnemyBase_C"))
    (for _array_element _outactors
      (bind _asaic_enemy_base (Utilities|Casting|CastToAIC_EnemyBase (AI|GetAIController _array_element)))
      (Default|SetStateasPassive _asaic_enemy_base))))

(event Input|KeyboardEvents|1
  (params (Key :type Key%20Structure :default "None"))
  ;[0.05098 0.05098 0.05098] debugging
  (:Pressed
    (bind _outactors (Actor|GetAllActorsOfClass "/Game/Enemies/Blueprints/BP_EnemyBase.BP_EnemyBase_C"))
    (for _array_element _outactors
      (bind _asaic_enemy_base (Utilities|Casting|CastToAIC_EnemyBase (AI|GetAIController _array_element)))
      (Default|SetStateasCombat _asaic_enemy_base))))

(fn GetRotationTowardsMouse
  (bind _returnvalue (Game|GetPlayerController 0))
  (bind _hitresult (Game|Player|GetHitResultUnderCursorbyChannel _returnvalue "TraceTypeQuery1" true))
  (bind (_targettedenemy _enemylocation) (CallFunction|GetTargettedEnemy))
  (return (.z (Math|Vector|SelectVector (+ (.yaw (Math|Rotator|FindLookatRotation (Transformation|GetActorLocation (Variables|Components|GetBP_PlayerCharacter)) (Math|Vector|SelectVector _enemylocation (.location _hitresult) (Utilities|IsValid _targettedenemy)))) 1.8e+02) (Math|Conversions|ToVector(Float) (.yaw (Math|Rotator|FindLookatRotation (Transformation|GetActorLocation (Variables|Components|GetBP_PlayerCharacter)) (Math|Vector|SelectVector _enemylocation (.location _hitresult) (Utilities|IsValid _targettedenemy))))) (== (.hitactor _hitresult) (Variables|Components|GetBP_PlayerCharacter))))))

(fn RotateTowardsMouse
  (bind _playerrotationz (CallFunction|GetRotationTowardsMouse))
  (Transformation|SetActorRotation (Variables|Components|GetBP_PlayerCharacter) (Math|Rotator|MakeRotator 0.0 0.0 _playerrotationz)))

(fn GetRotationTowardsEnemy
  (bind _returnvalue (Game|GetPlayerController 0))
  (bind _hitresult (Game|Player|GetHitResultUnderCursorbyChannel _returnvalue "TraceTypeQuery1" true))
  (bind (_targettedenemy _enemylocation) (Melee|GetClosestEnemy))
  (return (.z (Math|Vector|SelectVector (+ (.yaw (Math|Rotator|FindLookatRotation (Transformation|GetActorLocation (Variables|Components|GetBP_PlayerCharacter)) (Math|Vector|SelectVector _enemylocation (.location _hitresult) (Utilities|IsValid _targettedenemy)))) 1.8e+02) (Math|Conversions|ToVector(Float) (.yaw (Math|Rotator|FindLookatRotation (Transformation|GetActorLocation (Variables|Components|GetBP_PlayerCharacter)) (Math|Vector|SelectVector _enemylocation (.location _hitresult) (Utilities|IsValid _targettedenemy))))) (== (.hitactor _hitresult) (Variables|Components|GetBP_PlayerCharacter))))))

(fn RotateTowardsEnemy
  (bind _playerrotationz (Melee|GetRotationTowardsEnemy))
  (Transformation|SetActorRotation (Variables|Components|GetBP_PlayerCharacter) (Math|Rotator|MakeRotator 0.0 0.0 _playerrotationz)))

(fn GetTargettedEnemy
  (bind _targetenemy (Variables|TargetEnemy|GetTargetEnemy))
  (Utilities|IsValid _targetenemy
    (:Is%20Valid
      (return _targetenemy (Transformation|GetActorLocation _targetenemy)))
    (:Is%20Not%20Valid
      (return 0 "0, 0, 0"))))

(fn SetTargettedEnemy
  (params (TargettedEnemy :type Actor%20Object%20Reference))
  (Utilities|IsValid TargettedEnemy
    (:Is%20Valid
      (Variables|TargetEnemy|SetTargetEnemy TargettedEnemy))
    (:Is%20Not%20Valid
      (Variables|TargetEnemy|SetTargetEnemy 0))))

(fn GetClosestEnemy
  (bind _playerrotationz (CallFunction|GetRotationTowardsMouse))
  (bind _output_get (LocalVariables|SetFrontPoint (+ (Transformation|GetActorLocation (Variables|Components|GetBP_PlayerCharacter)) (* (Math|Vector|GetForwardVector (Math|Rotator|MakeRotator 0.0 0.0 _playerrotationz)) 1.4e+02))))
  (bind _outactors (Collision|SphereOverlapActors _output_get 9e+01 (Utilities|Array|MakeArray "ObjectTypeQuery3") "/Game/Enemies/Blueprints/BP_EnemyBase.BP_EnemyBase_C" (Utilities|Array|MakeArray (Variables|Components|GetBP_PlayerCharacter))))
  (Rendering|Debug|DrawDebugSphere (LocalVariables|GetFrontPoint) 0.0 12 "(R=1.000000,G=1.000000,B=1.000000,A=1.000000)" 1.0 1.0)
  (if (Utilities|Array|IsNotEmpty _outactors)
    (for _array_element _outactors
      (if (< (Math|Vector|Distance(Vector) (Transformation|GetActorLocation _array_element) (LocalVariables|GetFrontPoint)) (LocalVariables|GetClosestDistance))
        (LocalVariables|SetClosestDistance (Math|Vector|Distance(Vector) (Transformation|GetActorLocation _array_element) (LocalVariables|GetFrontPoint)))
        (LocalVariables|SetClosestEnemy _array_element)))
    (return (LocalVariables|GetClosestEnemy) (Transformation|GetActorLocation (LocalVariables|GetClosestEnemy)))
    (else
      (return 0 "0, 0, 0"))))

(fn CheckCanAttack
  (if (Variables|BPC_PlayerCombat_C|GetCanAttack (Variables|Default|GetBPC_PlayerCombat))
    (if (Variables|BPC_PlayerCombat_C|GetIsAttacking (Variables|Default|GetBPC_PlayerCombat))
      _
      (else
        (return true))))
  (return false))

(fn CheckCanReleaseAttack
  (if (Variables|BPC_PlayerCombat_C|GetCanReleaseAttack (Variables|Default|GetBPC_PlayerCombat))
    (return true)
    (else
      (return false))))

(fn ChangeWeaponType
  (bind _weapontype (Variables|WeaponType|GetWeaponType))
  (bind _weaponmeshes (Variables|WeaponType|GetWeaponMeshes))
  (bind _bpc_playercombat (Variables|Default|GetBPC_PlayerCombat))
  (bind _value (Utilities|Map|Find _weaponmeshes _weapontype))
  (if (Utilities|Map|Contains _weaponmeshes _weapontype)
    (Rendering|SetVisibility _value true false)
    (if (!= (Variables|BPC_PlayerCombat_C|GetPreviousWeapon _bpc_playercombat) _value)
      (Rendering|SetVisibility (Variables|BPC_PlayerCombat_C|GetPreviousWeapon _bpc_playercombat) false false)
      (Variables|BPC_PlayerCombat_C|SetPreviousWeapon _bpc_playercombat _value))
    (return)))

(fn HandleFinishedAttacking
  (bind _bpc_playercombat (Variables|Default|GetBPC_PlayerCombat))
  (Utilities|ToggleChildrenIsAttacking false)
  (Variables|BPC_PlayerCombat_C|SetCanAttack _bpc_playercombat true)
  (Variables|BPC_PlayerCombat_C|SetCanReleaseAttack _bpc_playercombat false)
  (Variables|AttackChecks|SetCanAttack true)
  (Variables|AttackChecks|SetCanReleaseAttack false)
  (Variables|WeaponType|SetWeaponType "NewEnumerator1")
  (CallFunction|ChangeWeaponType))