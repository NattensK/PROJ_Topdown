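; Player hook ability component: fires a hook projectile toward the mouse cursor and pulls the player to the enemy it hits.
; Pressing Q locks movement and turns the player toward the cursor; release spawns BP_ProjectileHook, which expires shortly if nothing is hit.
; On a hit, a looping timer accelerates the player toward the target with camera lag disabled.
; Finishing restores movement and re-enables the attack after a cooldown.
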(event Custom|SpawnProjectile
  (bind _bp_playercharacter (Variables|Default|GetBP_PlayerCharacter))
  (bind _bp_playercharacter_2 (Variables|Default|GetBP_PlayerCharacter))
  ;[0.05098 0.05098 0.05098] SpawnProjectile - starts when q is released
  (CallFunction|StopRotating)
  (bind _returnvalue (Game|SpawnActorfromClass "/Game/Projectile/BP_ProjectileHook.BP_ProjectileHook_C" (Transformation|GetWorldTransform (Variables|/Game/Player/Blueprints/BP_PlayerCharacter.BP_PlayerCharacter_C|GetHookShootPoint _bp_playercharacter)) "Undefined" "MultiplyWithRoot" _bp_playercharacter 2.7e+03 0.0 false (Utilities|Struct|MakeS_DamageInfo (Math|Random|RandomFloatinRange 7.0 2e+01) "NewEnumerator2" "NewEnumerator2" "NewEnumerator3" "NewEnumerator0" 0.75) false 0 0))
  (bind _output_get (Variables|Default|SetBP_Projectile_Hook _returnvalue))
  (Collision|IgnoreActorwhenMoving (Variables|/Script/Engine.Character|GetCapsuleComponent _bp_playercharacter_2) _output_get true)
  (Collision|IgnoreActorwhenMoving (Variables|/Game/Projectile/BP_ProjectileBase.BP_ProjectileBase_C|GetBoxCollision _output_get) _bp_playercharacter_2 true)
  (Utilities|FlowControl|Delay 0.4)
  (bind _bp_projectile_hook (Variables|Default|GetBP_Projectile_Hook)
    (:then
      (if (not (Variables|/Game/Projectile/BP_ProjectileBase.BP_ProjectileBase_C|GetHasCollided _bp_projectile_hook))
        (CallFunction|HookFinished)
        (Actor|DestroyActor _bp_projectile_hook)))
    (:else)))

(event Custom|RotateTowardsMouseLerp
  ;[0.05098 0.05098 0.05098] Rotate player to mouse location
  (bind _returnvalue (Utilities|Time|SetTimerbyEvent (delegate Custom|RotateTowardsMouseLerp) 0.01 true))
  (Transformation|SetActorRotation (Variables|Default|GetBP_PlayerCharacter) (Math|Rotator|MakeRotator 0.0 0.0 (Utilities|RotatetoMouseLocation))))

(event Custom|StopRotating
  ;[0.05098 0.05098 0.05098] Rotate player to mouse location
  (Utilities|Time|ClearandInvalidateTimerbyHandle (stale Custom|RotateTowardsMouseLerp _returnvalue)))

(event Custom|HookHit
  ;[0.05098 0.05098 0.05098] HookHit - starts when hook hit an enemy
  (bind _returnvalue (Utilities|Time|SetTimerbyEvent (delegate Custom|HookHit) 0.01 true))
  (Variables|HookHit|SetHookHitTimerHandle _returnvalue)
  (bind (_vinterpto _distance) (Utilities|LerpLocationtoEnemy))
  (if (<= _distance 2e+02)
    (Utilities|Time|ClearandInvalidateTimerbyHandle (Variables|HookHit|GetHookHitTimerHandle))
    (Variables|HookHit|SetHookHitTimer 0.0)
    (Variables|/Script/Engine.SpringArmComponent|SetbEnableCameraLag (Variables|/Game/Player/Blueprints/BP_PlayerCharacter.BP_PlayerCharacter_C|GetSpringArm (Variables|Default|GetBP_PlayerCharacter)) true)
    (CallFunction|HookFinished)
    (Utilities|FlowControl|Delay 0.1)
    (bind _bp_projectile_hook (Variables|Default|GetBP_Projectile_Hook)
      (:then
        (Actor|DestroyActor _bp_projectile_hook))
      (:else))
    (else
      (Transformation|SetActorLocation (Variables|Default|GetBP_PlayerCharacter) _vinterpto false false))))

(event Custom|HookFinished
  ;[0.05098 0.05098 0.05098] HookFinished - starts when hook hit nothing or when enemy got hit and player is close to enemy
  (Default|ToggleEnableMovementInput (Variables|Default|GetBP_PlayerCharacter) true true)
  (Default|FinishedAttacking (Variables|Default|GetBPC_PlayerCombat))
  ;;[0.05098 0.05098 0.05098] Can not attack with this ability until cooldown is finished
  (Utilities|FlowControl|Delay (Variables|Default|GetAttackCooldown))
  (Variables|/Game/Player/Blueprints/BPC_PlayerCombat.BPC_PlayerCombat_C|SetCanAttack (Variables|Default|GetBPC_PlayerHook) true))

(event Custom|HookAttack
  ;[0.05098 0.05098 0.05098] Attack - played when q is pressed
  (Variables|/Game/Player/Blueprints/BPC_PlayerCombat.BPC_PlayerCombat_C|SetIsAttacking (Variables|Default|GetBPC_PlayerHook) true)
  (Default|ToggleEnableMovementInput (Variables|Default|GetBP_PlayerCharacter) false false)
  (CallFunction|RotateTowardsMouseLerp)
  (Animation|Montage|PlayMontage (Variables|Default|GetPlayerMesh) "/Game/Characters/Mannequins/Animations/Bow_Animations/StandingEquipBow_UE_Montage.StandingEquipBow_UE_Montage" 0.7))

(event Custom|HookLanded
  (params (EnemyHit :type Actor%20Object%20Reference))
  ;[0.05098 0.05098 0.05098] HookLanded - starts when BP_ProjectileHook collides with something
  (bind _output_get (Variables|Default|SetTargetEnemy EnemyHit))
  (Variables|/Script/Engine.SpringArmComponent|SetbEnableCameraLag (Variables|/Game/Player/Blueprints/BP_PlayerCharacter.BP_PlayerCharacter_C|GetSpringArm (Variables|Default|GetBP_PlayerCharacter)) false)
  (Transformation|SetActorRotation (Variables|Default|GetBP_PlayerCharacter) (Math|Rotator|MakeRotator 0.0 0.0 (.yaw (Math|Rotator|FindLookatRotation (Transformation|GetActorLocation (Variables|Default|GetBP_PlayerCharacter)) (Transformation|GetActorLocation _output_get)))))
  (CallFunction|HookHit)
  (CallFunction|StopRotating))

(event EventBeginPlay
  ;[0.05098 0.05098 0.05098] Setup
  (|CallParentFunction))

(fn ApplyForceTimerFunction
  (params (TimerHandle :type Timer%20Handle%20Structure))
  (Variables|HookHit|SetHookHitTimerHandle TimerHandle)
  (bind _output_get (Variables|HookHit|SetHookHitTimer (+ 0.01 (Variables|HookHit|GetHookHitTimer))))
  (if (>= 0.0 _output_get)
    (return)
    (else
      (Utilities|Time|ClearandInvalidateTimerbyHandle (Variables|HookHit|GetHookHitTimerHandle))
      (Variables|HookHit|SetHookHitTimer 0.0))))

(fn CheckCanAttack
  (bind _canattack (|CallParentFunction))
  (if _canattack
    (if (Variables|/Game/Player/Blueprints/BPC_PlayerCombat.BPC_PlayerCombat_C|GetCanAttack (Variables|Default|GetBPC_PlayerHook))
      (return true)
      (else
        _)))
  (return false))

(fn CheckCanReleaseAttack
  (bind _canreleaseattack (|CallParentFunction))
  (if _canreleaseattack
    (if (Variables|/Game/Player/Blueprints/BPC_PlayerCombat.BPC_PlayerCombat_C|GetCanReleaseAttack (Variables|Default|GetBPC_PlayerHook))
      (return true)
      (else
        _)))
  (return false))

(fn HandleFinishedAttacking
  (|CallParentFunction))