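; Player melee component that runs sword attacks, with a montage combo on the ground and a single montage in the air.
; Each attack targets and turns toward the closest enemy and disables movement input.
; Ground attacks also lunge via timer-repeated normalized launches toward that enemy, or the cursor if none.
; Animation-triggered start and stop events run a looping socket-to-socket blade trace, damaging each actor once per swing.
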(event Custom|TriggerSwordTrace
  ;[0.05098 0.05098 0.05098] Ray traces weapon animation when melee attacking
  (bind _returnvalue (Utilities|Time|SetTimerbyEvent (delegate Custom|SwordTraceLoop) 0.01 true))
  (Variables|Default|SetswordTracingTimerHandle _returnvalue))

(event Custom|SwordTraceLoop
  (bind _actorhitbytrace (Variables|Default|GetactorHitByTrace))
  (bind _sword (Variables|Default|GetSword))
  ;[0.05098 0.05098 0.05098] Ray traces weapon animation when melee attacking
  (bind _outhits (Collision|MultiLineTraceByChannel (Transformation|GetSocketLocation _sword "start") (Transformation|GetSocketLocation _sword "end") "TraceTypeQuery1" false 0 "None"))
  (bind _array_element (Utilities|Array|ForEachLoopwithBreak _outhits)
    (:LoopBody
      (if (not (Utilities|Array|ContainsItem _actorhitbytrace (.HitActor (Collision|BreakHitResult _array_element))))
        (Utilities|Array|Add _actorhitbytrace (.HitActor (Collision|BreakHitResult _array_element)))
        (Class|BPIDamagable|DealDamage(Message) (.HitActor (Collision|BreakHitResult _array_element)) (Utilities|Struct|MakeS_DamageInfo 2e+01 "NewEnumerator1" "NewEnumerator1"))))))

(event Custom|StopSwordTrace
  ;[0.05098 0.05098 0.05098] Ray traces weapon animation when melee attacking
  (Utilities|Time|ClearandInvalidateTimerbyHandle (Variables|Default|GetswordTracingTimerHandle))
  (Utilities|Array|Clear (Variables|Default|GetactorHitByTrace)))

(event Custom|ApplyForce
  ;[0.05098 0.05098 0.05098] Apply force when melee attacking
  (CallFunction|ApplyForceStartTimer))

(event Custom|MeleeAttack
  ;[0.05098 0.05098 0.05098] Attack
  (if (not (== (Variables|Default|GetattackCount) 4))
    (bind (_targettedenemy _enemyloccation) (CallFunction|GetClosestEnemy))
    (Variables|Default|SetTargettedEnemy _targettedenemy)
    (Variables|Default|SetTargettedEnemyLocation _enemyloccation)
    (Default|ToggleDisableMovementInput (Variables|Default|GetBP_PlayerCharacterREF) true)
    (CallFunction|RotateTowardsEnemy)
    (if (AI|Components|NavMovement|IsMovingonGround (Variables|Default|GetCharacterMovement))
      (CallFunction|MeleeAttackonGround)
      (else
        (CallFunction|MeleeAttackinAir)))))

(event Custom|MeleeAttackOnGround
  ;[0.05098 0.05098 0.05098] Melee attack
  (Utilities|FlowControl|Sequence
    (:then_0
      (Animation|Montage|PlayMontage (Variables|Default|GetMesh) (Utilities|Array|Get(acopy) (Variables|Default|GetattackAnims) (Variables|Default|GetattackCount)) 2.0
        (:then
          (Math|Integer|IncrementInt (Variables|Default|GetattackCount)))
        (:OnCompleted
          (Variables|Default|SetattackCount 0 :!label _label)
          (CallFunction|FinishedAttacking)
          (Default|ToggleDisableMovementInput (Variables|Default|GetBP_PlayerCharacterREF) false))
        (:OnInterrupted
          (Utilities|FlowControl|RetriggerableDelay 3.0)
          (goto _label))))
    (:then_1
      (CallFunction|ApplyForce))))

(event Custom|ApplyForceStartTimer
  (bind _returnvalue (Game|GetPlayerController 0))
  (bind _playeractorref (Variables|Default|GetPlayerActorREF))
  (bind _applyforcestrength (Variables|Default|GetapplyForceStrength))
  (bind _targettedenemy (Variables|Default|GetTargettedEnemy))
  (bind _targettedenemylocation (Variables|Default|GetTargettedEnemyLocation))
  (bind _hitresult (Game|Player|GetHitResultUnderCursorbyChannel _returnvalue "TraceTypeQuery1" true))
  (bind _returnvalue_2 (Utilities|IsValid _targettedenemy))
  (bind _returnvalue_3 (Transformation|GetActorLocation _playeractorref))
  (bind _returnvalue_4 (- _targettedenemylocation _returnvalue_3))
  (bind _returnvalue_5 (- (.location _hitresult) _returnvalue_3))
  (bind _returnvalue_6 (Math|Vector|SelectVector _returnvalue_4 _returnvalue_5 _returnvalue_2))
  (bind _returnvalue_7 (Math|Vector|Normalize _returnvalue_6))
  (bind _returnvalue_8 (* _applyforcestrength _returnvalue_7))
  ;[0.05098 0.05098 0.05098] Apply force when melee attacking
  (bind _returnvalue_9 (Utilities|Time|SetTimerbyEvent (delegate Custom|ApplyForceStartTimer) 0.001 true))
  (CallFunction|ApplyForceTimerFunction _returnvalue_9)
  (Character|LaunchCharacter (Variables|Default|GetBP_PlayerCharacterREF) (Math|Vector|MakeVector (.x _returnvalue_8) (.y _returnvalue_8) 0.0) false false))

(event Custom|MeleeAttackInAir
  ;[0.05098 0.05098 0.05098] Melee attack
  (Animation|Montage|PlayMontage (Variables|Default|GetMesh) "/Game/Characters/Mannequins/Animations/Attack_Animations/SwordAndShieldAttack_UE_Montage.SwordAndShieldAttack_UE_Montage" 2.0
    (:OnCompleted
      _)
    (:OnInterrupted
      (Utilities|FlowControl|RetriggerableDelay 3.0)))
  (CallFunction|FinishedAttacking))

(event EventBeginPlay
  ;[0.05098 0.05098 0.05098] Setup
  (|CallParentFunction)
  (Variables|Default|SetSword (Variables|/Game/Player/Blueprints/BP_PlayerCharacter.BP_PlayerCharacter_C|GetSword (Variables|Default|GetBP_PlayerCharacterREF))))

(fn FinishedMeleeAttack)

(fn ApplyForceTimerFunction
  (params (TimerHandle :type Timer%20Handle%20Structure))
  (Variables|Default|SetapplyForceTimerHandle TimerHandle)
  (bind _output_get (Variables|Default|SetapplyForceTimer (+ 0.01 (Variables|Default|GetapplyForceTimer))))
  (if (>= (Variables|Default|GetapplyForceDuration) _output_get)
    (return)
    (else
      (Utilities|Time|ClearandInvalidateTimerbyHandle (Variables|Default|GetapplyForceTimerHandle))
      (Variables|Default|SetapplyForceTimer 0.0))))