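; Actor component that handles health, damage and death, broadcasting death, block and damage-response events.
; DealDamage routes through the CanBeDamaged macro, which checks death, invincibility and blocking, then subtracts health and fires responses on interruptible or forced hits.
; Helpers cache the skeletal meshes and materials of an actor and apply materials and an overlay to those meshes.
; Heal and the health and death getter functions are stubs returning defaults.
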(event Custom|SetAllMaterial
  (params (Materials :type Material%20Interface%20Object%20Reference) (OverlayMaterial :type Material%20Interface%20Object%20Reference))
  (for _array_element (Variables|Default|GetskeletalMeshes)
    (Rendering|Material|SetOverlayMaterial _array_element OverlayMaterial :!class /Script/Engine.MeshComponent)
    (for (_ _array_index) (Variables|Default|GetMaterials)
      (Rendering|Material|SetMaterial _array_element _array_index Materials))))

(event EventBeginPlay
  (Variables|Default|Sethealth (Variables|Default|GetmaxHealth)))

(event EventTick
  (params (DeltaSeconds :type Float%20%28single-precision%29)))

(fn GetAllMaterialsandMeshes
  (params (Actor :type Actor%20Object%20Reference))
  (for _array_element (Actor|GetComponentsByClass Actor "/Script/Engine.SkeletalMeshComponent")
    (Utilities|Array|Add (Variables|Default|GetskeletalMeshes) _array_element)
    (for _array_element_2 (Rendering|Material|GetMaterials _array_element)
      (Utilities|Array|Add (Variables|Default|GetMaterials) _array_element_2))))

(fn DealDamage
  (params (DamageInfo :type S%20Damage%20Info%20Structure))
  (bind (_damageamount _damagetype _damageresponse _shoulddamageinvincible _canbeblocked _canbeparried _shouldforceinterrupt) (Utilities|Struct|BreakS_DamageInfo DamageInfo))
  (Utilities|CanbeDamaged _shoulddamageinvincible _canbeblocked
    (:DoDamage
      (bind _output_get (Variables|Default|Sethealth (- (Variables|Default|Gethealth) _damageamount)))
      (Development|PrintString (Utilities|String|ToString(Float) _output_get))
      (if (<= _output_get 0.0)
        (Variables|Default|Setis%20Dead true)
        (Default|CallOnDeath)
        (return true)
        (elif (or (Variables|Default|GetisInterruptible) _shouldforceinterrupt)
          (Default|CallOnDamageResponse _damageresponse)
          (return true))))
    (:BlockDamage
      (Default|CallOnBlocked _canbeparried)
      (return false))
    (:NoDamage
      (return false))))

(fn GetCurrentHealth
  (return 0.0))

(fn GetMaxHealth
  (return 0.0))

(fn Heal
  (params (Amount :type Float%20%28double-precision%29))
  (return 0.0))

(fn IsDead
  (return false))