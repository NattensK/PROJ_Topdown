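; BP_DamagePopup is a short-lived actor that displays a damage amount through its DamagePopupWidget.
; On BeginPlay it passes DamageAmount to the widget, records its start location, and destroys itself after a one-second delay.
; The damage and health functions, such as DealDamage, Heal and IsDead, are stubs that only return default values or nothing.
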(event EventBeginPlay
  (Class|BPIDamagable|SetDamage(Message) (UserInterface|GetWidget (Variables|Default|GetDamagePopupWidget)) (Variables|Default|GetDamageAmount))
  (Variables|Default|SetStartPOS (Transformation|GetActorLocation))
  (Utilities|FlowControl|Delay 1.0)
  (Actor|DestroyActor))

(fn ConstructionScript)

(fn DealDamage
  (params (DamageInfo :type S%20Damage%20Info%20Structure))
  (return false))

(fn GetCurrentHealth
  (return 0.0))

(fn GetDamage
  (return 0.0))

(fn GetMaxHealth
  (return 0.0))

(fn Heal
  (params (Amount :type Float%20%28double-precision%29))
  (return 0.0))

(fn IsDead
  (return false))

(fn SetDamage
  (params (DamageAmount :type Float%20%28double-precision%29))
  (return))